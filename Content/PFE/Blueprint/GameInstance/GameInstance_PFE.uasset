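; Game instance for the PFE game that holds session joining, weapon choice and challenge progress state.
; It joins a selected session search result through the first player controller and toggles mutually exclusive Sword and Claw flags.
; A begin check marks the first challenge valid once its enemy kill count reaches the threshold.
; The replication callback for ChargingCrystals is empty.
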(event Custom|JoinToSelectedServer
  (params (SearchResult :type Blueprint%20Session%20Result%20Structure%20%28by%20ref%29))
  (|JoinSession (Game|GetPlayerController 0) SearchResult))

(event Custom|CheckOnBegin
  (Utilities|FlowControl|Sequence
    (:then_0
      (if (>= (Variables|Default|GetChallenge1EnemyKill) 1.0)
        (Variables|Default|SetChallenge1Valid true)))))

(event Custom|ChangeToClaw
  (Variables|Default|SetClaw true)
  (Variables|Default|SetSword false))

(event Custom|ChangeToSword
  (Variables|Default|SetSword true)
  (Variables|Default|SetClaw false))

(fn OnRepChargingCrystals)