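; VR multiplayer game mode that manages three enemy waves and their countdown timer.
; On BeginPlay it finds one spawner per wave and starts looping timers on all three at the EnemiesPerSeconds rate.
; Tick relies on one-second Delays to throttle GameInstance_PFE checks and decrement the clock stored there.
; Countdown resets the minutes according to the active wave, and running out of time only prints a message.
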(event Custom|Countdown
  (bind _spawnerw2 (Variables|Default|GetSpawnerW2))
  (bind _spawner3 (Variables|Default|GetSpawner3))
  (bind _gi (Variables|Default|GetGI))
  (bind _gi_2 (Variables|Default|GetGI))
  (bind _gi_3 (Variables|Default|GetGI))
  (Utilities|FlowControl|Sequence
    (:then_0
      (if (and (Variables|/Game/PFE/Blueprint/GameInstance/GameInstance_PFE.GameInstance_PFE_C|GetInW1 _gi_3) (not (Variables|Default|GetInTimer)))
        (Variables|/Game/PFE/Blueprint/GameInstance/GameInstance_PFE.GameInstance_PFE_C|SetMinute _gi_3 3.0)
        (Variables|Default|SetInTimer true)
        (if (<= (Variables|/Game/PFE/Blueprint/GameInstance/GameInstance_PFE.GameInstance_PFE_C|GetMinute _gi_2) -1.0) :!label _label
          (Development|PrintString "OUT OF TIME ENCULE")
          (Variables|Default|SetInTimer false))
        (elif (Math|Boolean|ANDBoolean (Variables|/Game/PFE/Blueprint/AI/AIGlobal/Spawner/EnemySpawnerW2.EnemySpawnerW2_C|GetCanSpawn _spawnerw2) (not (Variables|/Game/PFE/Blueprint/AI/AIGlobal/Spawner/EnemySpawnerW2.EnemySpawnerW2_C|GetEnd _spawnerw2)) (not (Variables|Default|GetInTimer)))
          (Variables|/Game/PFE/Blueprint/GameInstance/GameInstance_PFE.GameInstance_PFE_C|SetMinute _gi_3 4.0)
          (Variables|Default|SetInTimer true)
          (elif (Math|Boolean|ANDBoolean (Variables|/Game/PFE/Blueprint/AI/AIGlobal/Spawner/EnemySpawnerW3.EnemySpawnerW3_C|GetCanSpawn _spawner3) (not (Variables|/Game/PFE/Blueprint/AI/AIGlobal/Spawner/EnemySpawnerW3.EnemySpawnerW3_C|GetEnd _spawner3)) (not (Variables|Default|GetInTimer)))
            (Variables|/Game/PFE/Blueprint/GameInstance/GameInstance_PFE.GameInstance_PFE_C|SetMinute _gi_3 5.0)
            (Variables|Default|SetInTimer true)))))
    (:then_1
      (Utilities|FlowControl|Delay 1.0)
      (Variables|/Game/PFE/Blueprint/GameInstance/GameInstance_PFE.GameInstance_PFE_C|SetSecond _gi (- (Variables|/Game/PFE/Blueprint/GameInstance/GameInstance_PFE.GameInstance_PFE_C|GetSecond _gi) 1.0))
      (if (< (Variables|Default|GetSecond) 0)
        (Variables|/Game/PFE/Blueprint/GameInstance/GameInstance_PFE.GameInstance_PFE_C|SetMinute _gi (- (Variables|/Game/PFE/Blueprint/GameInstance/GameInstance_PFE.GameInstance_PFE_C|GetMinute _gi) 1.0))
        (Variables|/Game/PFE/Blueprint/GameInstance/GameInstance_PFE.GameInstance_PFE_C|SetSecond _gi_2 59.0)
        (goto _label)
        (else
          (goto _label))))))

(event EventTick
  (params (DeltaSeconds :type Float%20%28single-precision%29))
  (Utilities|FlowControl|Sequence
    (:then_0
      (Utilities|FlowControl|Delay 1.0)
      (Default|CheckonBegin (Variables|Default|GetGI)))
    (:then_1
      (CallFunction|Countdown))))

(event EventBeginPlay
  ;[1 1 1] WaveGestion
  (Utilities|FlowControl|Sequence
    (:then_0
      (bind _asgame_instance_pfe (Utilities|Casting|CastToGameInstance_PFE (Game|GetGameInstance)))
      (Variables|Default|SetGI _asgame_instance_pfe))
    (:then_1
      (Utilities|FlowControl|Sequence
        (:then_0
          (bind _outactors (Actor|GetAllActorsOfClass "/Game/PFE/Blueprint/AI/AIGlobal/Spawner/EnemySpawner.EnemySpawner_C"))
          (bind _output_get (Variables|Default|SetSpawner (Utilities|Array|Get(acopy) _outactors)))
          (Utilities|Time|SetTimerbyFunctionName _output_get "SpawnEnemy" (/ 1.0 (Variables|Default|GetEnemiesPerSeconds)) true))
        (:then_1
          (bind _outactors_2 (Actor|GetAllActorsOfClass "/Game/PFE/Blueprint/AI/AIGlobal/Spawner/EnemySpawnerW2.EnemySpawnerW2_C"))
          (bind _output_get_2 (Variables|Default|SetSpawnerW2 (Utilities|Array|Get(acopy) _outactors_2)))
          (Utilities|Time|SetTimerbyFunctionName _output_get_2 "Wave2" (/ 1.0 (Variables|Default|GetEnemiesPerSeconds)) true))
        (:then_2
          (bind _outactors_3 (Actor|GetAllActorsOfClass "/Game/PFE/Blueprint/AI/AIGlobal/Spawner/EnemySpawnerW3.EnemySpawnerW3_C"))
          (bind _output_get_3 (Variables|Default|SetSpawner3 (Utilities|Array|Get(acopy) _outactors_3)))
          (Utilities|Time|SetTimerbyFunctionName _output_get_3 "Wave3" (/ 1.0 (Variables|Default|GetEnemiesPerSeconds)) true))))))

(fn ConstructionScript)