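; Destructible pillar actor that loses its light and dissolves away when it is overlapped or hit.
; The trigger swaps two material slots to the dissolve material and destroys the PointLight, then P2 waits briefly before dissolving seven slots through timeline-driven dynamic material instances.
; Each timeline starts the next from its Update pin rather than Finished, so downstream instances are recreated every update.
; The last timeline destroys the actor when it finishes.
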(event OnComponentBeginOverlap(Pillar_DES_DM)
  (params (OverlappedComponent :type Primitive%20Component%20Object%20Reference) (OtherActor :type Actor%20Object%20Reference) (OtherComp :type Primitive%20Component%20Object%20Reference) (OtherBodyIndex :type Integer) (bFromSweep :type Boolean) (SweepResult :type Hit%20Result%20Structure%20%28by%20ref%29))
  (Utilities|FlowControl|Sequence
    (:then_0
      (CallFunction|P1))
    (:then_1
      (CallFunction|P2))))

(event OnComponentHit(Pillar_DES_DM)
  (params (HitComponent :type Primitive%20Component%20Object%20Reference) (OtherActor :type Actor%20Object%20Reference) (OtherComp :type Primitive%20Component%20Object%20Reference) (NormalImpulse :type Vector :default "0, 0, 0") (Hit :type Hit%20Result%20Structure%20%28by%20ref%29))
  (Utilities|FlowControl|Sequence
    (:then_0
      (CallFunction|P1))
    (:then_1
      (CallFunction|P2))))

(event Custom|P1
  (CallFunction|ChangeEmissive)
  (Components|DestroyComponent (Variables|Default|GetPointLight)))

(event Custom|P2
  (Utilities|FlowControl|Delay 1.5)
  (bind _returnvalue (Rendering|Material|CreateDynamicMaterialInstance (Variables|Default|GetPillar_DES_DM) 0 "/Game/PFE/Material/FX/Disint/PillarDissolve_Inst.PillarDissolve_Inst" "None" :!class /Script/Engine.PrimitiveComponent))
  (bind _newtrack_0 (Timeline|Timeline_0 Play)
    (:Update
      (Rendering|Material|SetScalarParameterValue _returnvalue "Amount" _newtrack_0 :!class /Script/Engine.MaterialInstanceDynamic)
      (bind _returnvalue_2 (Rendering|Material|CreateDynamicMaterialInstance (Variables|Default|GetPillar_DES_DM) 3 "/Game/PFE/Material/FX/Disint/PillarDissolve_Inst.PillarDissolve_Inst" "None" :!class /Script/Engine.PrimitiveComponent))
      (bind _newtrack_0_2 (Timeline|Timeline_1 Play)
        (:Update
          (Rendering|Material|SetScalarParameterValue _returnvalue_2 "amount" _newtrack_0_2 :!class /Script/Engine.MaterialInstanceDynamic)
          (bind _returnvalue_3 (Rendering|Material|CreateDynamicMaterialInstance (Variables|Default|GetPillar_DES_DM) 6 "/Game/PFE/Material/FX/Disint/PillarDissolve_Inst.PillarDissolve_Inst" "None" :!class /Script/Engine.PrimitiveComponent))
          (bind _newtrack_0_3 (Timeline|Timeline_2 Play)
            (:Update
              (Rendering|Material|SetScalarParameterValue _returnvalue_3 "amount" _newtrack_0_3 :!class /Script/Engine.MaterialInstanceDynamic)
              (bind _returnvalue_4 (Rendering|Material|CreateDynamicMaterialInstance (Variables|Default|GetPillar_DES_DM) 4 "/Game/PFE/Material/FX/Disint/PillarDissolve_Inst.PillarDissolve_Inst" "None" :!class /Script/Engine.PrimitiveComponent))
              (bind _newtrack_0_4 (Timeline|Timeline_3 Play)
                (:Update
                  (Rendering|Material|SetScalarParameterValue _returnvalue_4 "amount" _newtrack_0_4 :!class /Script/Engine.MaterialInstanceDynamic)
                  (bind _returnvalue_5 (Rendering|Material|CreateDynamicMaterialInstance (Variables|Default|GetPillar_DES_DM) 5 "/Game/PFE/Material/FX/Disint/PillarDissolve_Inst.PillarDissolve_Inst" "None" :!class /Script/Engine.PrimitiveComponent))
                  (bind _newtrack_0_5 (Timeline|Timeline_4 Play)
                    (:Update
                      (Rendering|Material|SetScalarParameterValue _returnvalue_5 "amount" _newtrack_0_5 :!class /Script/Engine.MaterialInstanceDynamic)
                      (bind _returnvalue_6 (Rendering|Material|CreateDynamicMaterialInstance (Variables|Default|GetPillar_DES_DM) 1 "/Game/PFE/Material/FX/Disint/PillarDissolve_Inst.PillarDissolve_Inst" "None" :!class /Script/Engine.PrimitiveComponent))
                      (bind _newtrack_0_6 (Timeline|Timeline_5 Play)
                        (:Update
                          (Rendering|Material|SetScalarParameterValue _returnvalue_6 "amount" _newtrack_0_6 :!class /Script/Engine.MaterialInstanceDynamic)
                          (bind _returnvalue_7 (Rendering|Material|CreateDynamicMaterialInstance (Variables|Default|GetPillar_DES_DM) 2 "/Game/PFE/Material/FX/Disint/PillarDissolve_Inst.PillarDissolve_Inst" "None" :!class /Script/Engine.PrimitiveComponent))
                          (bind _newtrack_0_7 (Timeline|Timeline_6 Play)
                            (:Update
                              (Rendering|Material|SetScalarParameterValue _returnvalue_7 "amount" _newtrack_0_7 :!class /Script/Engine.MaterialInstanceDynamic))
                            (:Finished
                              (Actor|DestroyActor))))))))))))))))

(event Collision|EventActorBeginOverlap
  (params (OtherActor :type Actor%20Object%20Reference))
  (Utilities|FlowControl|Sequence
    (:then_0
      (CallFunction|P1))
    (:then_1
      (CallFunction|P2))))

(fn ConstructionScript)

(fn ChangeEmissive
  (Rendering|Material|CreateDynamicMaterialInstance (Variables|Default|GetPillar_DES_DM) 1 "/Game/PFE/Material/FX/Disint/PillarDissolve_Inst.PillarDissolve_Inst" "None" :!class /Script/Engine.PrimitiveComponent)
  (Rendering|Material|CreateDynamicMaterialInstance (Variables|Default|GetPillar_DES_DM) 2 "/Game/PFE/Material/FX/Disint/PillarDissolve_Inst.PillarDissolve_Inst" "None" :!class /Script/Engine.PrimitiveComponent))