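; AI enemy character that hunts Player2, with movement held briefly after spawn as a wave-launch delay.
; Pawn sensing or Chase turns it toward a Player2 pawn and issues an AI move, which also enables firing.
; A looping timer spawns LaserIA shots while alive and player index 1 is in range.
; An empty magazine triggers a timed reload mirrored to the blackboard; an obsolete trace-based movement branch never runs.
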(event OnSeePawn(PawnSensing)
  (params (Pawn :type Pawn%20Object%20Reference))
  ;[1 1 1] Chase Event
  (bind _asplayer_2 (Utilities|Casting|CastToPlayer2 Pawn))
  (Variables|Default|SetNewVar_0_0 _asplayer_2)
  (Transformation|SetActorRotation (Math|Rotator|FindLookatRotation (Transformation|GetActorLocation) (Transformation|GetActorLocation _asplayer_2)))
  (Utilities|FlowControl|Sequence
    (:then_0
      (if true
        (AI|AIMoveTo self (Transformation|GetActorLocation _asplayer_2) _asplayer_2 1e+03 false
          (:then
            (Variables|Default|SetSee true)))))))

(event Custom|Reload
  ;[1 1 1] Reload Event
  (if (not (or (Variables|Default|GetIsReloading) (Variables|Default|GetIsdead_0)))
    (AI|Components|Blackboard|SetValueasBool (AI|GetBlackboard (Pawn|GetController)) (Utilities|Name|MakeLiteralName "isReloading") true)
    (Variables|Default|SetIsReloading true)
    (Utilities|FlowControl|Delay 2.5)
    (Variables|Default|SetAmmoInMag (Variables|Default|GetMaxAmmoInMag))
    (Variables|Default|SetIsReloading false)
    (AI|Components|Blackboard|SetValueasBool (AI|GetBlackboard (Pawn|GetController)) (Utilities|Name|MakeLiteralName "isReloading") false)))

(event Custom|Fire
  ;[1 1 1] Fire Events
  (if (and (>= (Variables|Default|GetLife) 1.0) (Variables|Default|GetSee))
    (if (== (Variables|Default|GetAmmoInMag) 0)
      (CallFunction|Reload)
      (elif (< (Math|Vector|VectorLength (- (Transformation|GetActorLocation (Game|Player|GetPlayerPawn 1)) (Transformation|GetActorLocation))) 2.5e+03)
        (Game|SpawnActorfromClass "/Game/PFE/Blueprint/BulletsOrWeapon/Bullets/LaserIA.LaserIA_C" (Transformation|GetWorldTransform (Variables|Default|GetArrow1)) "Undefined" 0 0)
        (Variables|Default|SetAmmoInMag (- (Variables|Default|GetAmmoInMag) 1))))))

(event Custom|Chase
  ;[1 1 1] Chase Event
  (bind _asplayer_2 (Utilities|Casting|CastToPlayer2 (stale OnSeePawn(PawnSensing) Pawn)))
  (Variables|Default|SetNewVar_0_0 _asplayer_2)
  (Transformation|SetActorRotation (Math|Rotator|FindLookatRotation (Transformation|GetActorLocation) (Transformation|GetActorLocation _asplayer_2)))
  (Utilities|FlowControl|Sequence
    (:then_0
      (if true
        (AI|AIMoveTo self (Transformation|GetActorLocation _asplayer_2) _asplayer_2 1e+03 false
          (:then
            (Variables|Default|SetSee true)))))))

(event EventBeginPlay
  ;[1 1 1] Set Timer Fire
  (Utilities|FlowControl|Sequence
    (:then_0
      (Utilities|Time|SetTimerbyFunctionName 0 "Fire" 0.5 true)
      (CallFunction|Chase))
    (:then_1
      (Components|Activation|Deactivate (Variables|Character|GetCharacterMovement))
      ;[1 1 1] Activate Wave
      (Utilities|FlowControl|Delay 2.0)
      (Development|PrintString "AntiJ2_Launch")
      (Components|Activation|Activate (Variables|Character|GetCharacterMovement) false))))

(fn ConstructionScript
  (|CallParentFunction))