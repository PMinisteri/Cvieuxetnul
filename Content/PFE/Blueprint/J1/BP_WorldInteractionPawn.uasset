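; VR motion-controller pawn, apparently Player 1, with grab/use, trace interaction, a weapon, a shield and a gesture spell.
; Per-hand interactor components handle input; Claw or Sword is chosen from GameInstance_PFE and swapped through a child actor.
; The spell menu reveals chained trigger volumes the left hand traces to arm a temporary shock spell, spawning a ShockWave on floor contact.
; Player 2 attach/energy logic and overheat handling look unfinished.
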(event OnComponentBeginOverlap(Spell1)
  (params (OverlappedComponent :type Primitive%20Component%20Object%20Reference) (OtherActor :type Actor%20Object%20Reference) (OtherComp :type Primitive%20Component%20Object%20Reference) (OtherBodyIndex :type Integer) (bFromSweep :type Boolean) (SweepResult :type Hit%20Result%20Structure%20%28by%20ref%29))
  ;[1 1 1] A changer / Decrocher le dynamic spell de la camera
  ;;[0.08557 1 0.06308] All step for Spell 1
  ;;;[0.08557 1 0.06308] Select a spell
  (if (and (Components|ComponentHasTag OtherComp "HandL") (Variables|SpellSystem|GetInSpellMenu))
    (Rendering|SetVisibility (Variables|Default|GetSpell1) false false)
    (Variables|SpellSystem|SetInSpellSystem true)
    (Rendering|SetVisibility (Variables|Default|GetBoxColliderSpell1) false false)
    (Rendering|SetVisibility (Variables|Default|GetAgar1%20%28changer%20le%20systeme) true false)))

(event OnComponentBeginOverlap(Agar1(changerlesysteme)
  (params (OverlappedComponent :type Primitive%20Component%20Object%20Reference) (OtherActor :type Actor%20Object%20Reference) (OtherComp :type Primitive%20Component%20Object%20Reference) (OtherBodyIndex :type Integer) (bFromSweep :type Boolean) (SweepResult :type Hit%20Result%20Structure%20%28by%20ref%29))
  ;[1 1 1] A changer / Decrocher le dynamic spell de la camera
  ;;[0.08557 1 0.06308] All step for Spell 1
  ;;;[0.08557 1 0.06308] P1 Spell System
  (Utilities|FlowControl|Sequence
    (:then_0
      _)
    (:then_1
      (Utilities|FlowControl|Delay 1.5)
      (Variables|Spell1|SetBeginSpell1 true)))
  (if (and (Components|ComponentHasTag OtherComp "HandL") (Variables|SpellSystem|GetInSpellSystem))
    (Rendering|SetVisibility (Variables|Default|GetAgarLimit) true false)
    (Variables|Spell1|SetP1Spell1 true)))

(event OnComponentEndOverlap(AgarLimit)
  (params (OverlappedComponent :type Primitive%20Component%20Object%20Reference) (OtherActor :type Actor%20Object%20Reference) (OtherComp :type Primitive%20Component%20Object%20Reference) (OtherBodyIndex :type Integer))
  ;[1 1 1] A changer / Decrocher le dynamic spell de la camera
  ;;[0.08557 1 0.06308] All step for Spell 1
  ;;;[0.08557 1 0.06308] P1 Spell System
  (if (and (Variables|Spell1|GetBeginSpell1) (Components|ComponentHasTag OtherComp "HandL"))
    (Rendering|SetVisibility (Variables|Default|GetAgar1%20%28changer%20le%20systeme) false false)
    (Variables|Spell1|SetP1Spell1 false)
    (if (not (Variables|Spell1|GetP2Spell1))
      (Variables|SpellSystem|SetInSpellSystem false)
      (Variables|SpellSystem|SetInSpellMenu false)
      (Rendering|SetVisibility (Variables|Default|GetP1_2) false false)
      (Variables|Spell1|SetBeginSpell1 false))))

(event OnComponentBeginOverlap(Agar2)
  (params (OverlappedComponent :type Primitive%20Component%20Object%20Reference) (OtherActor :type Actor%20Object%20Reference) (OtherComp :type Primitive%20Component%20Object%20Reference) (OtherBodyIndex :type Integer) (bFromSweep :type Boolean) (SweepResult :type Hit%20Result%20Structure%20%28by%20ref%29))
  ;[1 1 1] A changer / Decrocher le dynamic spell de la camera
  ;;[0.08557 1 0.06308] All step for Spell 1
  ;;;[0.08557 1 0.06308] P2 Spell System
  (if (Math|Boolean|ANDBoolean (Components|ComponentHasTag OtherComp "HandL") (Variables|Spell1|GetP1Spell1) (Variables|SpellSystem|GetInSpellSystem))
    (Variables|Spell1|SetP2Spell1 true)
    (Rendering|SetVisibility (Variables|Default|GetP1_3) true false)))

(event OnComponentBeginOverlap(SphereRange)
  (params (OverlappedComponent :type Primitive%20Component%20Object%20Reference) (OtherActor :type Actor%20Object%20Reference) (OtherComp :type Primitive%20Component%20Object%20Reference) (OtherBodyIndex :type Integer) (bFromSweep :type Boolean) (SweepResult :type Hit%20Result%20Structure%20%28by%20ref%29))
  ;[1 0 0.04632] Useless (for a moment)
)

(event OnComponentEndOverlap(AgarLimit2)
  (params (OverlappedComponent :type Primitive%20Component%20Object%20Reference) (OtherActor :type Actor%20Object%20Reference) (OtherComp :type Primitive%20Component%20Object%20Reference) (OtherBodyIndex :type Integer))
  ;[1 1 1] A changer / Decrocher le dynamic spell de la camera
  ;;[0.08557 1 0.06308] All step for Spell 1
  ;;;[0.08557 1 0.06308] P2 Spell System
  (if (Components|ComponentHasTag OtherComp "HandL")
    (Rendering|SetVisibility (Variables|Default|GetAgarLimit2) false false)
    (Variables|Spell1|SetP2Spell1 false)
    (if (not (Variables|Spell1|GetEndSpell1))
      (Variables|SpellSystem|SetInSpellSystem false)
      (Variables|SpellSystem|SetInSpellMenu false)
      (Rendering|SetVisibility (Variables|Default|GetAgarFin) false false))))

(event OnComponentBeginOverlap(ShockSpell)
  (params (OverlappedComponent :type Primitive%20Component%20Object%20Reference) (OtherActor :type Actor%20Object%20Reference) (OtherComp :type Primitive%20Component%20Object%20Reference) (OtherBodyIndex :type Integer) (bFromSweep :type Boolean) (SweepResult :type Hit%20Result%20Structure%20%28by%20ref%29))
  (if (Variables|Spell1|GetHasShock)
    (if (Actor|ActorHasTag OtherActor "Floor")
      (Game|SpawnActorfromClass "/Game/PFE/Blueprint/BulletsOrWeapon/DynamicSpells/ShockWave.ShockWave_C" (Math|Transform|MakeTransform (Transformation|GetWorldLocation (Variables|Default|GetShockSpell)) "0, 0, 0" "1,1,1") "Undefined" 0 0))))

(event OnComponentBeginOverlap(AgarFin)
  (params (OverlappedComponent :type Primitive%20Component%20Object%20Reference) (OtherActor :type Actor%20Object%20Reference) (OtherComp :type Primitive%20Component%20Object%20Reference) (OtherBodyIndex :type Integer) (bFromSweep :type Boolean) (SweepResult :type Hit%20Result%20Structure%20%28by%20ref%29))
  ;[1 1 1] A changer / Decrocher le dynamic spell de la camera
  ;;[0.08557 1 0.06308] All step for Spell 1
  ;;;[0.08557 1 0.06308] LastPhaseSpell
  (if (Math|Boolean|ANDBoolean (Variables|Spell1|GetP2Spell1) (Variables|SpellSystem|GetInSpellSystem) (Components|ComponentHasTag OtherComp "HandL"))
    (Variables|Spell1|SetEndSpell1 true)
    (CallFunction|SpawnShockSpell)
    (Rendering|SetVisibility (Variables|Default|GetP1_2) false false)
    (Variables|SpellSystem|SetInSpellMenu false)
    (Variables|SpellSystem|SetInSpellSystem false)
    (Rendering|SetVisibility (Variables|Default|GetAgarFin) false false)
    (Utilities|FlowControl|Delay 1e+01)
    (Variables|Spell1|SetEndSpell1 false)
    (Variables|Spell1|SetP1Spell1 false)
    (Variables|Spell1|SetP2Spell1 false)
    (Rendering|SetVisibility (Variables|Default|GetAgar1%20%28changer%20le%20systeme) false false)
    (Variables|Spell1|SetBeginSpell1 false)))

(event OnComponentEndOverlap(Sphere1)
  (params (OverlappedComponent :type Primitive%20Component%20Object%20Reference) (OtherActor :type Actor%20Object%20Reference) (OtherComp :type Primitive%20Component%20Object%20Reference) (OtherBodyIndex :type Integer))
  ;[1 0 0.04632] Useless (for a moment)
)

(event Custom|SelectSword
  ;[1 1 1] ChangeWeapon System
  (Default|ChangetoSword (Variables|Default|GetGI))
  (CallFunction|GotoSword))

(event Custom|GiveEnergyP2
  (bind _p2 (Variables|Default|GetP2))
  ;[1 0.7725 0] Not Use for now
  (Variables|/Game/PFE/Blueprint/J2/Player2.Player2_C|SetEnergy _p2 (+ (Variables|/Game/PFE/Blueprint/J2/Player2.Player2_C|GetEnergy _p2) 25.0)))

(event Custom|ShieldSpawn
  (bind _shieldp1 (Variables|Default|GetShieldP1))
  ;[0 1 0.1765] Shield SPARTAAAAA
  ;;[0 1 0.1765] Shield Spawn / Despawn Custom Event
  (if (Variables|Default|GetInShield)
    _
    (else
      (Variables|Default|SetInShield true)
      (ChildActorComponent|SetChildActorClass _shieldp1 "/Game/PFE/Blueprint/BulletsOrWeapon/Weapons/ShieldP1.ShieldP1_C")
      (Utilities|FlowControl|Delay 45.0)))
  (ChildActorComponent|SetChildActorClass _shieldp1 0)
  (Variables|Default|SetInShield false))

(event Custom|SpellUnClose
  ;[0.2601 1 0.9801] Custom Event Spells List
  (Rendering|SetVisibility (Variables|Default|GetSpell1) false false))

(event Custom|SpawnShockSpell
  (bind _shockspell (Variables|Default|GetShockSpell))
  ;[0.8409 1 0.01124] SpawnWeapon
  (Rendering|ToggleVisibility _shockspell false)
  (Variables|Spell1|SetHasShock true)
  (Transformation|SetWorldLocation _shockspell (Transformation|GetWorldLocation (Variables|Default|GetHandR)) false false)
  (Utilities|FlowControl|Delay 5.0)
  (CallFunction|DespawnShockSpell))

(event Custom|GoToSword
  ;[1 1 1] SpawnWeapon System
  (ChildActorComponent|SetChildActorClass (Variables|Default|GetWeaponClaw) "/Game/PFE/Blueprint/BulletsOrWeapon/Weapons/BP_Sword.BP_Sword_C"))

(event Custom|DecreaseOverheat
  ;[1 0 0.04632] Useless (for a moment)
  (Variables|Default|SetOverheat (- (Variables|Default|GetOverheat) 2.0)))

(event Custom|ChangeWeapon
  ;[1 1 1] ChangeWeapon Event
  (if (Variables|Weapons|GetClaw)
    (ChildActorComponent|SetChildActorClass (Variables|Default|GetWeaponClaw) "/Game/PFE/Blueprint/BulletsOrWeapon/Weapons/BP_Claw.BP_Claw_C")
    (elif (Variables|Weapons|GetSword)
      (ChildActorComponent|SetChildActorClass (Variables|Default|GetWeaponClaw) "/Game/PFE/Blueprint/BulletsOrWeapon/Weapons/BP_Sword.BP_Sword_C"))))

(event Custom|GoToClaw
  ;[1 1 1] SpawnWeapon System
  (ChildActorComponent|SetChildActorClass (Variables|Default|GetWeaponClaw) "/Game/PFE/Blueprint/BulletsOrWeapon/Weapons/BP_Claw.BP_Claw_C"))

(event Custom|SelectClaw
  ;[1 1 1] ChangeWeapon System
  (Default|ChangetoClaw (Variables|Default|GetGI))
  (CallFunction|GotoSword))

(event Custom|DespawnShockSpell
  ;[0.8409 1 0.01124] SpawnWeapon
  (Rendering|ToggleVisibility (Variables|Default|GetShockSpell) false)
  (Variables|Spell1|SetHasShock false))

(event Custom|FreezeOverheat
  (if (>= (Variables|Survive|GetTPHeat) 1)
    (Utilities|FlowControl|Delay 1.0)
    (Variables|Survive|SetTPHeat (+ (Variables|Survive|GetTPHeat) 10))))

(event Custom|SpellUnOpen
  ;[0.2601 1 0.9801] Custom Event Spells List
  (if (not (and (Variables|Spell1|GetEndSpell1) (Variables|Default|GetInShield)))
    (Rendering|SetVisibility (Variables|Default|GetSpell1) true false)))

(event Custom|Attach
  (bind _l_hand_sphere (Variables|Default|GetL_Hand_Sphere))
  (bind _returnvalue (Transformation|GetWorldRotation _l_hand_sphere))
  (bind _returnvalue_2 (Transformation|GetWorldLocation _l_hand_sphere))
  ;[1 0 0.04632] Useless (for a moment)
  (Transformation|SetActorLocation (stale _asplayer_2) (Math|Vector|MakeVector (- (.x _returnvalue_2) 35.0) (+ (.y _returnvalue_2) 5.0) (.z _returnvalue_2)) false false)
  (Transformation|SetActorRotation (stale _asplayer_2) (Math|Rotator|MakeRotator (- (.roll _returnvalue) 9e+01) (.pitch _returnvalue) (.yaw _returnvalue))))

(event EventBeginPlay
  (bind _returnvalue (Game|GetGameInstance))
  ;[0.912 0.3965 1] Event Begin Play
  ;;[1 1 1] Setup Trace Interactor
  (bind _returnvalue_2 (Game|SpawnActorfromClass "/Game/VRTemplate/ExampleContent/VR_Trace_Interaction/Blueprints/BP_TraceVisualiser.BP_TraceVisualiser_C" (Math|Transform|MakeTransform "0, 0, 0") "Undefined" 0 1.0 "8.000000,0.800000,0.800000" 0))
  (Default|Setup (Variables|Default|GetBP_TraceInteractor_L) _returnvalue_2 self "NewEnumerator2" true (Variables|Default|GetWidgetInteraction))
  (bind _returnvalue_3 (Game|SpawnActorfromClass "/Game/VRTemplate/ExampleContent/VR_Trace_Interaction/Blueprints/BP_TraceVisualiser.BP_TraceVisualiser_C" (Math|Transform|MakeTransform "0, 0, 0") "Undefined" 0 1.0 "8.000000,0.800000,0.800000" 0))
  (Default|Setup (Variables|Default|GetBP_TraceInteractor_R) _returnvalue_3 self "NewEnumerator2" true (Variables|Default|GetWidgetInteraction))
  ;;[1 1 1] Setup World Interactor
  (Default|Setup (Variables|Default|GetBPC_WorldInteractor_L) (Variables|Default|GetL_Hand_Sphere))
  (Default|Setup (Variables|Default|GetBPC_WorldInteractor_R) (Variables|Default|GetR_Hand_Sphere))
  ;;[1 1 1] Set Floor Level
  (Class|HeadMountedDisplayFunctionLibrary|SetTrackingOrigin "Floor")
  ;;[1 1 1] LastStep
  (bind _asgame_instance_pfe (Utilities|Casting|CastToGameInstance_PFE _returnvalue))
  (Utilities|Casting|CastToGameInstance_PFE _returnvalue)
  (bind _output_get (Variables|Default|SetGI _asgame_instance_pfe))
  (if (Variables|/Game/PFE/Blueprint/GameInstance/GameInstance_PFE.GameInstance_PFE_C|GetClaw _output_get)
    (ChildActorComponent|SetChildActorClass (Variables|Default|GetWeaponClaw) "/Game/PFE/Blueprint/BulletsOrWeapon/Weapons/BP_Claw.BP_Claw_C")
    (elif (Variables|/Game/PFE/Blueprint/GameInstance/GameInstance_PFE.GameInstance_PFE_C|GetSword _output_get)
      (ChildActorComponent|SetChildActorClass (Variables|Default|GetWeaponClaw) "/Game/PFE/Blueprint/BulletsOrWeapon/Weapons/BP_Sword.BP_Sword_C"))))

(event EventEndPlay
  (params (EndPlayReason :type EEndPlayReason%20Enum :default "Destroyed"))
  ;[1 1 1] Event End Play
  (|DestroySession))

(event EventTick
  (params (DeltaSeconds :type Float%20%28single-precision%29))
  (Utilities|FlowControl|Delay 0.2)
  (Utilities|FlowControl|Sequence
    (:then_0
      (CallFunction|FreezeOverheat))))

(event Input|ActionEvents|InputActionDynamicSpell
  (params (Key :type Key%20Structure))
  ;[1 1 1] A changer / Decrocher le dynamic spell de la camera
  ;;[0.08557 1 0.06308] Spell Selection
  ;;;[0.08557 1 0.06308] Launch Spell Menu
  (:Pressed
    (if (Variables|SpellSystem|GetInSpellMenu)
      (CallFunction|SpellUnClose)
      (Variables|SpellSystem|SetInSpellMenu false)
      (if (Variables|SpellSystem|GetInSpellSystem)
        (Variables|SpellSystem|SetInSpellSystem false)
        (Rendering|SetVisibility (Variables|Default|GetBoxColliderSpell1) false false))
      (else
        (Variables|SpellSystem|SetInSpellMenu true)
        (CallFunction|SpellUnOpen)))))

(event Input|ActionEvents|InputActionPickupLeft
  (params (Key :type Key%20Structure))
  (bind _bpc_worldinteractor_l (Variables|Default|GetBPC_WorldInteractor_L))
  ;[0.08557 1 0.06308] Pickup
  (:Pressed
    (Default|PickupPressed _bpc_worldinteractor_l)
    (Default|DragStart _bpc_worldinteractor_l))
  (:Released
    (Default|PickupReleased _bpc_worldinteractor_l)
    (Default|DragStop _bpc_worldinteractor_l)))

(event Input|ActionEvents|InputActionPickupRight
  (params (Key :type Key%20Structure))
  (bind _bpc_worldinteractor_r (Variables|Default|GetBPC_WorldInteractor_R))
  ;[0.08557 1 0.06308] Pickup
  (:Pressed
    (Default|PickupPressed _bpc_worldinteractor_r)
    (Default|DragStart _bpc_worldinteractor_r))
  (:Released
    (Default|PickupReleased _bpc_worldinteractor_r)
    (Default|DragStop _bpc_worldinteractor_r)))

(event Input|ActionEvents|InputActionShieldP1
  (params (Key :type Key%20Structure))
  ;[0 1 0.1765] Shield SPARTAAAAA
  ;;[0 1 0.1765] Use Shield
  (:Pressed
    (CallFunction|ShieldSpawn)))

(event Input|KeyboardEvents|MotionControllerLeftFaceButton1
  (params (Key :type Key%20Structure))
  (bind _bp_traceinteractor_l (Variables|Default|GetBP_TraceInteractor_L))
  ;[0.06772 0.2163 1] Activate trace
  (:Pressed
    (Default|ActivateEventDown _bp_traceinteractor_l))
  (:Released
    (Default|ActivateEventUp _bp_traceinteractor_l)
    (Variables|Survive|SetTPHeat (- (Variables|Survive|GetTPHeat) 10))))

(event Input|KeyboardEvents|MotionControllerRightFaceButton1
  (params (Key :type Key%20Structure))
  ;[0.06772 0.2163 1] Activate trace
)

(event Input|KeyboardEvents|MotionControllerRightFaceButton2
  (params (Key :type Key%20Structure))
  ;[0.8409 1 0.01124] SpawnWeapon
)

(event Input|KeyboardEvents|MotionControllerLeftTrigger
  (params (Key :type Key%20Structure))
  (bind _bpc_worldinteractor_l (Variables|Default|GetBPC_WorldInteractor_L))
  ;[0.08557 1 0.06308] Use objects
  (:Pressed
    (Default|UsePressed _bpc_worldinteractor_l))
  (:Released
    (Default|UseReleased _bpc_worldinteractor_l)))

(event Input|KeyboardEvents|MotionControllerRightTrigger
  (params (Key :type Key%20Structure))
  (bind _bpc_worldinteractor_r (Variables|Default|GetBPC_WorldInteractor_R))
  ;[0.08557 1 0.06308] Use objects
  (:Pressed
    (Default|UsePressed _bpc_worldinteractor_r))
  (:Released
    (Default|UseReleased _bpc_worldinteractor_r)))

(fn ConstructionScript)