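; SelectChallenge is a HUB Blueprint that reveals a challenge element when a hand touches it.
; On BeginPlay it casts and caches the PFE game instance.
; When an actor tagged "Hand" begins overlapping Sphere1, it shows the Challenge1 component if the game instance's Challenge1Valid flag is false.
; Only the first challenge is handled, and nothing hides it again.
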(event OnComponentBeginOverlap(Sphere1)
  (params (OverlappedComponent :type Primitive%20Component%20Object%20Reference) (OtherActor :type Actor%20Object%20Reference) (OtherComp :type Primitive%20Component%20Object%20Reference) (OtherBodyIndex :type Integer) (bFromSweep :type Boolean) (SweepResult :type Hit%20Result%20Structure%20%28by%20ref%29))
  (if (Actor|ActorHasTag OtherActor "Hand")
    (if (not (Variables|/Game/PFE/Blueprint/GameInstance/GameInstance_PFE.GameInstance_PFE_C|GetChallenge1Valid (Variables|Default|GetGI)))
      (Rendering|SetVisibility (Variables|Default|GetChallenge1) true false))))

(event EventBeginPlay
  (bind _asgame_instance_pfe (Utilities|Casting|CastToGameInstance_PFE (Game|GetGameInstance)))
  (Variables|Default|SetGI _asgame_instance_pfe))

(fn ConstructionScript)