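; Multiplayer objective actor: a crystal that AI lasers damage, ending in a loss when its health runs out.
; Overlaps with actors tagged LaserIA subtract basic damage from ObjectifLife, which is stored in GameInstance_PFE.
; Falling health thresholds recolor the Cube mesh orange, then red, through dynamic material instances created on each qualifying hit.
; At zero, the Loose event sets the game instance's Life to zero.
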(event Custom|Loose
  (Variables|/Game/PFE/Blueprint/GameInstance/GameInstance_PFE.GameInstance_PFE_C|SetLife (Variables|Default|GetGI) 0.0))

(event EventBeginPlay
  (bind _asgame_instance_pfe (Utilities|Casting|CastToGameInstance_PFE (Game|GetGameInstance)))
  (Variables|Default|SetGI _asgame_instance_pfe))

(event Collision|EventActorBeginOverlap
  (params (OtherActor :type Actor%20Object%20Reference))
  (bind _gi (Variables|Default|GetGI))
  (if (Actor|ActorHasTag OtherActor "LaserIA")
    (Variables|/Game/PFE/Blueprint/GameInstance/GameInstance_PFE.GameInstance_PFE_C|SetObjectifLife _gi (- (Variables|/Game/PFE/Blueprint/GameInstance/GameInstance_PFE.GameInstance_PFE_C|GetObjectifLife _gi) (Variables|Default|GetDamageTakenByBasic)))
    (if (<= (Variables|/Game/PFE/Blueprint/GameInstance/GameInstance_PFE.GameInstance_PFE_C|GetObjectifLife _gi) 5e+02)
      (bind _returnvalue (Rendering|Material|CreateDynamicMaterialInstance (Variables|Default|GetCube) 0 "/Game/PFE/Blueprint/BulletsOrWeapon/Bullets/Materials/CristalLifeMat.CristalLifeMat" "" :!class /Script/Engine.PrimitiveComponent))
      (Rendering|Material|SetVectorParameterValue _returnvalue "BaseColor" "(R=1.000000,G=0.232668,B=0.000000,A=1.000000)" :!class /Script/Engine.MaterialInstanceDynamic)
      (if (<= (Variables|/Game/PFE/Blueprint/GameInstance/GameInstance_PFE.GameInstance_PFE_C|GetObjectifLife _gi) 2e+02)
        (bind _returnvalue_2 (Rendering|Material|CreateDynamicMaterialInstance (Variables|Default|GetCube) 0 "/Game/PFE/Blueprint/BulletsOrWeapon/Bullets/Materials/CristalLifeMat.CristalLifeMat" "" :!class /Script/Engine.PrimitiveComponent))
        (Rendering|Material|SetVectorParameterValue _returnvalue_2 "BaseColor" "(R=1.000000,G=0.000000,B=0.000000,A=1.000000)" :!class /Script/Engine.MaterialInstanceDynamic)
        (if (<= (Variables|/Game/PFE/Blueprint/GameInstance/GameInstance_PFE.GameInstance_PFE_C|GetObjectifLife (Variables|Default|GetGI)) 0.0)
          (CallFunction|Loose))))))

(fn ConstructionScript)